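; BP_PlayerCharacter is the player-controlled character, with axis-driven walking and camera look, a click attack against a boss, and a respawn.
; Left click runs Attack, which finds a BP_BossAI actor and sends fixed damage to its AI controller, with no range or aim check.
; Tick watches Health and, at zero or below, teleports the character to its BeginPlay position and resets Health.
; DisableMovement and EnableMovement events toggle walking.
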(event `self.ReceiveBeginPlay`
  (set `self.StartPosition` (`self.K2_GetActorLocation`)))

(event `self.ReceiveTick`
  (params (DeltaSeconds :type "Float (single-precision)"))
  (if (<= (`self.Health`) 0.0)
    (`self.K2_SetActorLocation` (`self.StartPosition`) false true)
    (set `self.Health` 10.0)))

(event `InputAxis|MoveForward`
  (params (AxisValue :type "Float (single-precision)"))
  (`self.AddMovementInput` (`self.GetActorForwardVector`) AxisValue))

(event `InputAxis|MoveRight`
  (params (AxisValue :type "Float (single-precision)"))
  (`self.AddMovementInput` (`self.GetActorRightVector`) AxisValue))

(event `InputAxis|Turn`
  (params (AxisValue :type "Float (single-precision)"))
  (`self.AddControllerYawInput` AxisValue))

(event `InputAxis|LookUp`
  (params (AxisValue :type "Float (single-precision)"))
  (`self.AddControllerPitchInput` AxisValue))

(event `Key|LeftMouseButton`
  (params (Key :type "Key Structure"))
  (:`Pressed`
    (`self.Attack`)))

(event `/Game/BossAI/BP_Interfaces/BPI_TargetCharacter.DisableMovement`
  (`CharacterMovementComponent.DisableMovement` (`self.CharacterMovement`)))

(event `/Game/BossAI/BP_Interfaces/BPI_TargetCharacter.EnableMovement`
  (`CharacterMovementComponent.SetMovementMode` (`self.CharacterMovement`) "MOVE_Walking" 0))

(fn `Attack`
  (bind _returnvalue (`GameplayStatics.GetActorOfClass` "/Game/BossAI/BP_BossAI.BP_BossAI_C"))
  (message `/Game/BossAI/BP_Interfaces/BPI_Damageable.TakeDamage` (`AIBlueprintHelperLibrary.GetAIController` _returnvalue) 10.0))

(fn `UserConstructionScript`)