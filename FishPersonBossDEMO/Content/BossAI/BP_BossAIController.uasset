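; AI controller for a boss that tracks its health and switches between idle, chase, melee-range and long-range behavior trees against player 0.
; Each tick it updates Blackboard health, then picks a tree from target distance, with low health selecting the second attack variant.
; Once out of idle, a delayed random roll decides whether a distant target triggers a long-range sequence or a chase.
; Tree switches stop the running logic and skip the already active tree.
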(event `self.ReceiveBeginPlay`
  ;[1 1 1] Initialise Blackboard values, target player, and default state
  (set `self.CurrentHealth` (`self.MaxHealth`))
  (set `self.TargetPlayer` (`GameplayStatics.GetPlayerCharacter` 0))
  (bind _blackboardcomponent (`self.UseBlackboard` "/Game/BossAI/BB_Boss.BB_Boss"))
  (`BlackboardComponent.SetValueAsFloat` _blackboardcomponent (`self.FullHealth`) (`self.MaxHealth`))
  (`BlackboardComponent.SetValueAsFloat` _blackboardcomponent (`self.SelfHealth`) (`self.CurrentHealth`))
  (`self.RunBehaviorTree` "/Game/BossAI/BehaviourTrees/BT_BossIdle.BT_BossIdle")
  (set `self.ActiveBehaviorTree` "/Game/BossAI/BehaviourTrees/BT_BossIdle.BT_BossIdle"))

(event `/Game/BossAI/BP_Interfaces/BPI_Damageable.TakeDamage`
  (params (Damage :type "Float (double-precision)"))
  ;[1 1 1] TakeDamageEvent
  (bind _output_get (set `self.CurrentHealth` (- (`self.CurrentHealth`) Damage)))
  (`self.OnHealthChanged` _output_get))

(event `Event SwitchBehaviourTree`
  (params (NewBehaviorTree :type "BehaviorTree Object Reference"))
  ;[1 1 1] Switch Behaviour Tree
  (bind _activebehaviortree (`self.ActiveBehaviorTree`)
    (:`then`
      (if (not (== NewBehaviorTree _activebehaviortree))
        (`BrainComponent.StopLogic` (`self.BrainComponent`) "")
        (`self.RunBehaviorTree` NewBehaviorTree :!label _label)
        (set `self.OldBehaviourTree` (`self.ActiveBehaviorTree`))
        (bind _output_get (set `self.ActiveBehaviorTree` NewBehaviorTree))
        (`KismetSystemLibrary.PrintString` (`KismetSystemLibrary.GetDisplayName` _output_get))))
    (:`else`
      (goto _label))))

(event `self.ReceiveTick`
  (params (DeltaSeconds :type "Float (single-precision)"))
  (bind _lowhealth (`self.IsLowHealth`))
  (bind _activebehaviortree (`self.ActiveBehaviorTree`))
  ;[1 1 1] Update on tick
  (`|ExecutionSequence`
    (:`then_0`
      (`BlackboardComponent.SetValueAsFloat` (`AIBlueprintHelperLibrary.GetBlackboard` null) (`self.SelfHealth`) (`self.CurrentHealth`))
      (if (`self.Is Target Near`)
        (if _lowhealth
          (`self.Event SwitchBehaviourTree` "/Game/BossAI/BehaviourTrees/BT_AtckSqnce2.BT_AtckSqnce2")
          (else
            (`self.Event SwitchBehaviourTree` "/Game/BossAI/BehaviourTrees/BT_AtckSqnce1.BT_AtckSqnce1")))
        (elif (!= (`self.ActiveBehaviorTree`) "/Game/BossAI/BehaviourTrees/BT_BossIdle.BT_BossIdle")
          (if (`self.Is Target Far`)
            (if (== (`self.RangeCondition`) 4)
              (set `self.RangeCondition` 0)
              (if _lowhealth
                (`self.Event SwitchBehaviourTree` "/Game/BossAI/BehaviourTrees/BT_LongRange2.BT_LongRange2")
                (else
                  (`self.Event SwitchBehaviourTree` "/Game/BossAI/BehaviourTrees/BT_LongRange1.BT_LongRange1")))
              (elif (not (or (== _activebehaviortree "/Game/BossAI/BehaviourTrees/BT_LongRange1.BT_LongRange1") (== _activebehaviortree "/Game/BossAI/BehaviourTrees/BT_LongRange2.BT_LongRange2")))
                (`self.Event SwitchBehaviourTree` "/Game/BossAI/BehaviourTrees/BT_BossChase.BT_BossChase")))))))
    (:`then_1`
      (`KismetSystemLibrary.Delay` 2.0)
      (if (!= (`self.ActiveBehaviorTree`) "/Game/BossAI/BehaviourTrees/BT_BossIdle.BT_BossIdle")
        (set `self.RangeCondition` (`KismetMathLibrary.RandomIntegerInRange` 0 4))))))

(fn `Is Target Far`
  (returns (IsFar :type Boolean))
  (return (>= (`self.GetDistanceTo` (`self.K2_GetPawn`) (`self.TargetPlayer`)) 1000.0)))

(fn `Is Target Near`
  (returns (InRange :type Boolean))
  (return (<= (`self.GetDistanceTo` (`self.K2_GetPawn`) (`self.TargetPlayer`)) 550.0)))

(fn `IsLowHealth`
  (returns (LowHealth :type Boolean))
  (return (< (`self.CurrentHealth`) 80.0)))

(fn `UserConstructionScript`)