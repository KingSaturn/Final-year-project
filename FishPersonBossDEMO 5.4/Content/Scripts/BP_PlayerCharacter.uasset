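; Player character Blueprint with axis-driven movement and look, plus a left-click attack against the boss.
; Attack finds a BP_BossAI through GetActorOfClass and sends Damage to its AI controller via TakeDamageMessage, with no range or hit check.
; DisableMovement and EnableMovement events switch character movement off and back to Walking.
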(event `InputAxis|MoveForward`
  (params (AxisValue :type "Float (single-precision)"))
  (`self.AddMovementInput` (`self.GetActorForwardVector`) AxisValue))

(event `InputAxis|MoveRight`
  (params (AxisValue :type "Float (single-precision)"))
  (`self.AddMovementInput` (`self.GetActorRightVector`) AxisValue))

(event `InputAxis|Turn`
  (params (AxisValue :type "Float (single-precision)"))
  (`self.AddControllerYawInput` AxisValue))

(event `InputAxis|LookUp`
  (params (AxisValue :type "Float (single-precision)"))
  (`self.AddControllerPitchInput` AxisValue))

(event `Key|LeftMouseButton`
  (params (Key :type "Key Structure"))
  (:`Pressed`
    (`self.Attack` (`self.Damage`))))

(event `/Game/BossAI/BP_Interfaces/BPI_TargetCharacter.DisableMovement`
  (`CharacterMovementComponent.DisableMovement` (`self.CharacterMovement`)))

(event `/Game/BossAI/BP_Interfaces/BPI_TargetCharacter.EnableMovement`
  (`CharacterMovementComponent.SetMovementMode` (`self.CharacterMovement`) "MOVE_Walking" 0))

(fn `Attack`
  (params (Damage :type "Float (double-precision)"))
  (bind _returnvalue (`GameplayStatics.GetActorOfClass` "/Game/BossAI/BP_BossAI.BP_BossAI_C"))
  (message `/Game/BossAI/BP_Interfaces/BPI_Damageable.TakeDamage` (`AIBlueprintHelperLibrary.GetAIController` _returnvalue) Damage))

(fn `UserConstructionScript`)