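; BP_BossAI is the boss actor blueprint, which shows a health bar widget kept in sync with its health.
; On BeginPlay it casts to BP_BossAIController, seeds W_Healthbar with max and current health, and binds OnHealthChanged to update the bar.
; Each Tick it turns the HealthBar component toward the player controller's location, using only X and Y so the bar stays upright.
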(event `self.ReceiveBeginPlay`
  ;[1 1 1] Set Widget Values
  (bind _asbp_boss_aicontroller (cast `/Game/BossAI/BP_BossAIController` (`AIBlueprintHelperLibrary.GetAIController` self)))
  (bind _output_get (set `self.As BP Boss AIController` _asbp_boss_aicontroller))
  (bind _asw_healthbar (cast `/Game/Widgets/W_Healthbar` (`WidgetComponent.GetWidget` (`self.HealthBar`))))
  (bind _output_get_2 (set `self.As W Healthbar` _asw_healthbar))
  (`/Game/Widgets/W_Healthbar.SetMaxHealth` _output_get_2 (`/Game/BossAI/BP_BossAIController.MaxHealth` _output_get))
  (`/Game/Widgets/W_Healthbar.SetCurrentHealth` _output_get_2 (`/Game/BossAI/BP_BossAIController.CurrentHealth` _output_get))
  (add `/Game/BossAI/BP_BossAIController.OnHealthChanged` _output_get (delegate `OnHealthChanged`)))

(event `OnHealthChanged`
  (params (NewHealth :type "Float (double-precision)"))
  ;[1 1 1] Set Widget Values
  (`/Game/Widgets/W_Healthbar.SetCurrentHealth` (stale `self.ReceiveBeginPlay` _output_get_2) NewHealth))

(event `self.ReceiveTick`
  (params (DeltaSeconds :type "Float (single-precision)"))
  (bind (_returnvalue_x _returnvalue_y) (`KismetMathLibrary.BreakVector` (`self.K2_GetActorLocation`)))
  (bind (_returnvalue_x_2 _returnvalue_y_2) (`KismetMathLibrary.BreakVector` (`self.K2_GetActorLocation` (`GameplayStatics.GetPlayerController` 0))))
  ;[1 1 1] Set Widget rotation
  (`SceneComponent.K2_SetWorldRotation` (`self.HealthBar`) (`KismetMathLibrary.FindLookAtRotation` (`KismetMathLibrary.MakeVector` _returnvalue_x _returnvalue_y) (`KismetMathLibrary.MakeVector` _returnvalue_x_2 _returnvalue_y_2)) false false))

(fn `UserConstructionScript`)